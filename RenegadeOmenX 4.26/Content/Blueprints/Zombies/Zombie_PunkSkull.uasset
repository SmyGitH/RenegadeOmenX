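; Punk skull zombie enemy Blueprint that handles taking damage, stumbling and dying.
; Any damage is subtracted from Health, then CheckAlive picks the branch.
; A true result, despite the name, stops the AI brain logic and destroys the actor after a delay; false plays the stumble montage if the mesh is not already playing.
; MeleeAttack only calls the parent implementation.
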(event Game|Damage|EventAnyDamage
  (params (Damage :type Float%20%28single-precision%29) (DamageType :type Damage%20Type%20Object%20Reference) (InstigatedBy :type Controller%20Object%20Reference) (DamageCauser :type Actor%20Object%20Reference))
  (Variables|Default|SetHealth (- (Variables|Default|GetHealth) Damage))
  (bind _dead (CallFunction|CheckAlive))
  (if _dead
    (AI|Logic|StopLogic (Variables|/Script/AIModule.AIController|GetBrainComponent (AI|GetAIController self)) "")
    (Utilities|FlowControl|Delay 5.0)
    (Actor|DestroyActor)
    (elif (not (Audio|Components|Audio|IsPlaying (Variables|Character|GetMesh)))
      (Animation|Montage|PlayMontage (Variables|Character|GetMesh) (Variables|Default|GetZombieStumble)))))

(event EventBeginPlay
  (|CallParentFunction) ; This node is disabled and will not be called.\nDrag off pins to build functionality.
)

(event EventMeleeAttack
  (|CallParentFunction))

(fn ConstructionScript
  (|CallParentFunction))