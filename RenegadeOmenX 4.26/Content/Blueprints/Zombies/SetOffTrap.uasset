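; Car noise trap for the zombie game that goes off when the first-person player overlaps its Box trigger.
; If the player's SetOffTrap flag is clear and CarNoise is silent, it sets the flag, plays the sound and reports an AI noise event at its location.
; It then calls FloodSpawn on every FloodSpawnPoint cached at BeginPlay, passing the audio component and player.
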(event OnComponentBeginOverlap(Box)
  (params (OverlappedComponent :type Primitive%20Component%20Object%20Reference) (OtherActor :type Actor%20Object%20Reference) (OtherComp :type Primitive%20Component%20Object%20Reference) (OtherBodyIndex :type Integer) (bFromSweep :type Boolean) (SweepResult :type Hit%20Result%20Structure%20%28by%20ref%29))
  (bind _asfirst_person_character (Utilities|Casting|CastToFirstPersonCharacter OtherActor))
  (if (not (Variables|/Game/Blueprints/FirstPersonBP/Blueprints/FirstPersonCharacter.FirstPersonCharacter_C|GetsetOffTrap _asfirst_person_character))
    (if (not (Audio|Components|Audio|IsPlaying (Variables|Default|GetCarNoise)))
      (Variables|/Game/Blueprints/FirstPersonBP/Blueprints/FirstPersonCharacter.FirstPersonCharacter_C|SetsetOffTrap _asfirst_person_character true)
      (bind _carnoise (CallFunction|PlaySound))
      (Class|AISenseHearing|ReportNoiseEvent (Transformation|GetActorLocation) 1.0 _asfirst_person_character 3e+03 "None")
      (for _array_element (Variables|Default|GetFlood%20Points)
        (Default|FloodSpawn _array_element _carnoise _asfirst_person_character)
        (Development|PrintString "isSpawning")))))

(event EventBeginPlay
  (bind _outactors (Actor|GetAllActorsOfClass "/Game/Blueprints/Zombies/FloodSpawnPoint.FloodSpawnPoint_C"))
  (Variables|Default|SetFlood%20Points _outactors)
  (Audio|Components|Audio|Stop (Variables|Default|GetCarNoise)))

(event Collision|EventActorBeginOverlap
  (params (OtherActor :type Actor%20Object%20Reference)))

(event EventTick
  (params (DeltaSeconds :type Float%20%28single-precision%29)))

(fn ConstructionScript)

(fn PlaySound
  (bind _carnoise (Variables|Default|GetCarNoise))
  (Audio|Components|Audio|Play _carnoise 0.5)
  (return _carnoise))