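; Zombie enemy character that melee-attacks the player and reacts to damage by stumbling or dying.
; MeleeAttack plays a montage whose notify sphere-traces at the hand's MeleeSocket, damaging and reporting a damage event if it hits the player.
; AnyDamage lowers Health; CheckAlive, which returns true at zero or below despite its name, triggers ragdoll, AI logic stop and delayed destruction after a montage completes.
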(event OnSystemFinished(Blood)
  (params (PSystem :type Niagara%20Component%20Object%20Reference))
  (Components|Activation|SetActive PSystem false false))

(event Game|Damage|EventAnyDamage
  (params (Damage :type Float%20%28single-precision%29) (DamageType :type Damage%20Type%20Object%20Reference) (InstigatedBy :type Controller%20Object%20Reference) (DamageCauser :type Actor%20Object%20Reference))
  (bind _mesh (Variables|Character|GetMesh))
  (Variables|Default|SetHealth (- (Variables|Default|GetHealth) Damage))
  (bind _dead (CallFunction|CheckAlive))
  (if _dead
    (Animation|Montage|PlayMontage _mesh 0
      (:OnCompleted
        (Physics|SetSimulatePhysics _mesh true)
        (AI|Logic|StopLogic (Variables|/Script/AIModule.AIController|GetBrainComponent (AI|GetAIController self)) "")
        (Utilities|FlowControl|Delay 5.0)
        (Actor|DestroyActor)))
    (elif (not (Audio|Components|Audio|IsPlaying (Variables|Character|GetMesh)))
      (Animation|Montage|PlayMontage (Variables|Character|GetMesh) (Variables|Default|GetZombieStumble)))))

(event EventBeginPlay
  (bind _asfirst_person_character (Utilities|Casting|CastToFirstPersonCharacter (Game|GetPlayerCharacter 0)))
  (Variables|Default|SetPlayerRef _asfirst_person_character)
  (Components|Activation|SetActive (Variables|Default|GetBlood) false false))

(event EventMeleeAttack
  (bind _mesh (Variables|Character|GetMesh))
  (bind _returnvalue (Transformation|GetSocketLocation _mesh "MeleeSocket"))
  (Animation|Montage|PlayMontage _mesh (Variables|Default|GetZombieAttack)
    (:OnNotifyBegin
      (bind _outhit (Collision|SphereTraceByChannel _returnvalue _returnvalue 1e+02 "TraceTypeQuery2" false 0 "Persistent"))
      (if (== (.hitactor _outhit) (Variables|Default|GetPlayerRef))
        (Class|AISenseDamage|ReportDamageEvent (.hitactor _outhit) self 0.0 (.tracestart _outhit))
        (Game|Damage|ApplyDamage (.hitactor _outhit) (Variables|Default|GetDamage) 0 0)))))

(fn ConstructionScript)

(fn CheckAlive
  (bind _health (Variables|Default|GetHealth))
  (bind _returnvalue (<= _health 0.0))
  (if _returnvalue
    (return _returnvalue)
    (else
      (return _returnvalue))))