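; Slot-based inventory component that stores item stacks and opens or closes the inventory window.
; Adding a stackable item tops up a partial stack of the same class, recursing through AddToInventory for overflow; otherwise it takes the first empty slot.
; PrepareInventory resizes the slot array and refreshes item data from class defaults on BeginPlay and before opening.
; ToggleInventory centres the window on the RenegadeController's HUD canvas, switches input mode and cursor, and clears tooltips on close.
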(event EventBeginPlay
  (CallFunction|PrepareInventory))

(event EventTick
  (params (DeltaSeconds :type Float%20%28single-precision%29)))

(fn ToggleInventory
  (bind _returnvalue (Game|GetPlayerController 0))
  (bind _returnvalue_2 (Game|GetPlayerController 0))
  (bind _inventorywindow (Variables|Default|GetInventoryWindow)
    (:then
      (bind _foundwidgets (Widget|GetAllWidgetsOfClass "/Game/Blueprints/FirstPersonBP/Blueprints/HUD/InventoryUI/InventoryToolTip.InventoryToolTip_C" false))
      (Widget|RemovefromParent _foundwidgets)
      (Widget|RemovefromParent _inventorywindow)
      (Variables|Default|SetInventoryWindow 0)
      (Input|SetInputModeGameOnly _returnvalue)
      (Variables|/Script/Engine.PlayerController|SetbShowMouseCursor _returnvalue false))
    (:else
      (CallFunction|PrepareInventory)
      (bind _returnvalue_3 (UserInterface|CreateWidget "/Game/Blueprints/FirstPersonBP/Blueprints/HUD/InventoryUI/InventoryWindow.InventoryWindow_C" 0 self))
      (Variables|Default|SetInventoryWindow _returnvalue_3)
      (bind _asrenegade_controller (Utilities|Casting|CastToRenegadeController (Game|GetPlayerController 0)))
      (bind _returnvalue_4 (Class|CanvasPanel|AddChildtoCanvas (Variables|/Game/Blueprints/FirstPersonBP/Blueprints/HUD/InventoryUI/InventoryHUD.InventoryHUD_C|GetHUDCanvas (Variables|/Game/Blueprints/FirstPersonBP/Blueprints/RenegadeController.RenegadeController_C|GetHUDWidget _asrenegade_controller)) (Variables|Default|GetInventoryWindow)))
      (Class|CanvasPanelSlot|SetAutoSize _returnvalue_4 true)
      (Class|CanvasPanelSlot|SetAlignment _returnvalue_4 "(X=0.500000,Y=0.500000)")
      (Class|CanvasPanelSlot|SetAnchors _returnvalue_4 (Utilities|Struct|MakeAnchors "(X=0.500000,Y=0.500000)" "(X=0.500000,Y=0.500000)"))
      (Class|CanvasPanelSlot|SetPosition _returnvalue_4 (Variables|Default|GetPosition))
      (Input|SetInputModeUIOnly _returnvalue_2 (Variables|Default|GetInventoryWindow) "LockAlways")
      (Variables|/Script/Engine.PlayerController|SetbShowMouseCursor _returnvalue_2 true))))

(fn AddtoInventory
  (params (ContentToAdd :type Slot%20Structure%20Structure))
  (if (.isstackable (.itemstructure ContentToAdd))
    (bind _stackindex (Utilities|HasPartialStack ContentToAdd)
      (:True
        (bind _success (CallFunction|AddtoStack ContentToAdd _stackindex))
        (LocalVariables|SetisSuccesful _success))
      (:False
        (bind _success_2 (CallFunction|CreateStack ContentToAdd :!label _label))
        (LocalVariables|SetisSuccesful _success_2)))
    (else
      (goto _label)))
  (return (LocalVariables|GetisSuccesful)))

(fn PrepareInventory
  (Utilities|Array|Resize (Variables|Default|GetInventory) (Variables|Default|GetNumberOfSlots))
  (for (_array_element _array_index) (Variables|Default|GetInventory)
    (if (!= 0 (.Class (Utilities|Struct|BreakItemStructure (.itemstructure _array_element))))
      (Utilities|Array|SetArrayElem (Variables|Default|GetInventory) _array_index (Utilities|Struct|MakeSlotStructure (.ItemStructure (Utilities|GetClassDefaults (.Class (Utilities|Struct|BreakItemStructure (.itemstructure _array_element))))) (.quantity _array_element))))))

(fn CreateStack
  (params (Content :type Slot%20Structure%20Structure))
  (bind (_array_element _array_index) (Utilities|Array|ForEachLoopwithBreak (Variables|Default|GetInventory) :!label _label)
    (:LoopBody
      (if (<= (.quantity _array_element) 0)
        (LocalVariables|SetHasSpace true)
        (LocalVariables|SetIdentifiedIndex _array_index)
        (goto _label Break)))
    (:Completed
      (if (LocalVariables|GetHasSpace)
        (Utilities|Array|SetArrayElem (Variables|Default|GetInventory) (LocalVariables|GetIdentifiedIndex) Content)
        (return (LocalVariables|GetHasSpace))
        (else
          (return false))))))

(fn AddtoStack
  (params (Contents :type Slot%20Structure%20Structure) (Slot%20Index :type Integer))
  (bind _inventory (Variables|Default|GetInventory))
  (bind _inventory_2 (Variables|Default|GetInventory))
  (bind _maxstacksize (Utilities|Struct|BreakItemStructure (.itemstructure Contents)))
  (bind _output (Utilities|Array|Get(acopy) _inventory Slot%20Index))
  (bind _output_2 (Utilities|Array|Get(acopy) _inventory_2 Slot%20Index))
  (bind _output_get (LocalVariables|SetCurrentQuantity (.quantity _output)))
  (if (> (+ (.Quantity (Utilities|Struct|BreakSlotStructure Contents)) _output_get) (.maxstacksize (.itemstructure _output)))
    (Utilities|Array|SetArrayElem _inventory_2 Slot%20Index (Utilities|Struct|MakeSlotStructure (.itemstructure Contents) _maxstacksize))
    (CallFunction|AddtoInventory (Utilities|Struct|MakeSlotStructure (.itemstructure Contents) (- (.quantity Contents) (- _maxstacksize (LocalVariables|GetCurrentQuantity)))))
    (else
      (Utilities|Array|SetArrayElem _inventory_2 Slot%20Index (Utilities|Struct|MakeSlotStructure (.itemstructure _output_2) (+ (.quantity _output_2) (.quantity Contents))))))
  (return true))