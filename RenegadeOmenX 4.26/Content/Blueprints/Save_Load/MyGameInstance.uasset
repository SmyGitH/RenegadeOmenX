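; Game instance that owns the save game, persisting the first-person player's progress and inventory across sessions.
; On init or LoadGame it loads the save slot, or creates a fresh save object if none exists.
; Save and load functions copy data between the character and that object, with AutoSave wrapping the save and ClearSaveData deleting the slot.
; A LoadLevel event forwards level names to a smooth level-load call.
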(event Custom|Load%20Game
  (bind _returnvalue (SaveGame|DoesSaveGameExist (Variables|Default|GetSaveSlotName)))
  (if _returnvalue
    (bind _returnvalue_2 (SaveGame|LoadGamefromSlot (Variables|Default|GetSaveSlotName)))
    (bind _assave_game_object (Utilities|Casting|CastToSaveGameObject _returnvalue_2))
    (Variables|Default|SetSaveGameData _assave_game_object)
    (else
      (bind _returnvalue_3 (SaveGame|CreateSaveGameObject "/Game/Blueprints/Save_Load/SaveGameObject.SaveGameObject_C"))
      (Variables|Default|SetSaveGameData _returnvalue_3))))

(event Custom|LoadLevel
  (params (Level%20Name :type Name))
  (Default|CallSmoothLoadLevel Level%20Name))

(event EventInit
  (bind _returnvalue (SaveGame|DoesSaveGameExist (Variables|Default|GetSaveSlotName)))
  (if _returnvalue
    (bind _returnvalue_2 (SaveGame|LoadGamefromSlot (Variables|Default|GetSaveSlotName)))
    (bind _assave_game_object (Utilities|Casting|CastToSaveGameObject _returnvalue_2))
    (Variables|Default|SetSaveGameData _assave_game_object)
    (else
      (bind _returnvalue_3 (SaveGame|CreateSaveGameObject "/Game/Blueprints/Save_Load/SaveGameObject.SaveGameObject_C"))
      (Variables|Default|SetSaveGameData _returnvalue_3))))

(fn SavePlayerData
  (bind _savegamedata (Variables|Default|GetSaveGameData))
  (bind _asfirst_person_character (Utilities|Casting|CastToFirstPersonCharacter (Game|GetPlayerCharacter 0)))
  (bind _output_get (LocalVariables|SetPlayer _asfirst_person_character))
  (Variables|/Game/Blueprints/Save_Load/SaveGameObject.SaveGameObject_C|SetPlayerData _savegamedata (Utilities|Struct|MakePlayerSaveData (Variables|/Game/Blueprints/FirstPersonBP/Blueprints/FirstPersonCharacter.FirstPersonCharacter_C|GetProgress _output_get) (Variables|/Game/Blueprints/Inventory/InventoryComponent.InventoryComponent_C|GetInventory (Variables|/Game/Blueprints/FirstPersonBP/Blueprints/FirstPersonCharacter.FirstPersonCharacter_C|GetInventoryComponent _output_get))))
  (SaveGame|SaveGametoSlot _savegamedata (Variables|Default|GetSaveSlotName))
  (Development|PrintString "Saved"))

(fn LoadPlayerData
  (bind _savegamedata (Variables|Default|GetSaveGameData))
  (bind _playerdata (Variables|/Game/Blueprints/Save_Load/SaveGameObject.SaveGameObject_C|GetPlayerData _savegamedata))
  (bind _asfirst_person_character (Utilities|Casting|CastToFirstPersonCharacter (Game|GetPlayerCharacter 0)))
  (bind _output_get (LocalVariables|SetPlayer _asfirst_person_character))
  (Variables|/Game/Blueprints/FirstPersonBP/Blueprints/FirstPersonCharacter.FirstPersonCharacter_C|SetProgress _output_get (.progress _playerdata))
  (Variables|/Game/Blueprints/Inventory/InventoryComponent.InventoryComponent_C|SetInventory (Variables|/Game/Blueprints/FirstPersonBP/Blueprints/FirstPersonCharacter.FirstPersonCharacter_C|GetInventoryComponent _output_get) (.inventory _playerdata)))

(fn ClearSaveData
  (SaveGame|DeleteGameinSlot (Variables|Default|GetSaveSlotName)))

(fn AutoSave
  (CallFunction|SavePlayerData))