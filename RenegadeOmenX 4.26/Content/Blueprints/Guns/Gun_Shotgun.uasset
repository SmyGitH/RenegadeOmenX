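; Shotgun weapon Blueprint, a child of a parent gun class that handles the core shooting, firing and reload logic.
; On BeginPlay it loads its ammo and clip values from the player's stored Shotgun struct.
; Starting to shoot calls FireBullet once after the parent logic.
; FireBullet and ReloadGun run the parent version, then write the gun's state back to the player's Shotgun and CurrentWeapon structs.
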(event EventBeginPlay
  (bind _player_ref (Variables|Default|GetPlayer%20ref))
  (bind _shotgun (Variables|/Game/Blueprints/FirstPersonBP/Blueprints/FirstPersonCharacter.FirstPersonCharacter_C|GetShotgun _player_ref))
  (|CallParentFunction)
  (Variables|Default|SetAmmoCurrent (.ammocurrent _shotgun))
  (Variables|Default|SetAmmoMax (.ammomax _shotgun))
  (Variables|Default|SetClipSize (.clipsize _shotgun)))

(event Collision|EventActorBeginOverlap
  (params (OtherActor :type Actor%20Object%20Reference))
  (|CallParentFunction OtherActor) ; This node is disabled and will not be called.\nDrag off pins to build functionality.
)

(event EventTick
  (params (DeltaSeconds :type Float%20%28single-precision%29))
  (|CallParentFunction DeltaSeconds) ; This node is disabled and will not be called.\nDrag off pins to build functionality.
)

(event EventStartShooting
  (|CallParentFunction)
  (CallFunction|FireBullet))

(event EventStopShooting
  (|CallParentFunction))

(fn ConstructionScript
  (|CallParentFunction))

(fn ReloadGun
  (bind _player_ref (Variables|Default|GetPlayer%20ref))
  (|CallParentFunction)
  (bind _output_get (Variables|/Game/Blueprints/FirstPersonBP/Blueprints/FirstPersonCharacter.FirstPersonCharacter_C|SetShotgun _player_ref (Utilities|Struct|MakeGunVariables "Gun_Shotgun_C" (Variables|Default|GetAmmoCurrent) (Variables|Default|GetAmmoMax) (Variables|Default|GetThumbnail) (Variables|Default|GetClipSize))))
  (Variables|/Game/Blueprints/FirstPersonBP/Blueprints/FirstPersonCharacter.FirstPersonCharacter_C|SetCurrentWeapon _player_ref _output_get))

(fn FireBullet
  (bind _player_ref (Variables|Default|GetPlayer%20ref))
  (|CallParentFunction)
  (bind _output_get (Variables|/Game/Blueprints/FirstPersonBP/Blueprints/FirstPersonCharacter.FirstPersonCharacter_C|SetShotgun _player_ref (Utilities|Struct|MakeGunVariables "Gun_Shotgun_C" (Variables|Default|GetAmmoCurrent) (Variables|Default|GetAmmoMax) (Variables|Default|GetThumbnail) (Variables|Default|GetClipSize))))
  (Variables|/Game/Blueprints/FirstPersonBP/Blueprints/FirstPersonCharacter.FirstPersonCharacter_C|SetCurrentWeapon _player_ref _output_get))