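; Grenade launcher gun Blueprint, a child weapon class that fires once each time shooting starts.
; BeginPlay loads current ammo, max ammo and clip size from the player's GrenadeLauncher record.
; FireBullet and ReloadGun run the parent logic, then write the ammo state back to that record and copy it to CurrentWeapon, so the player's data stays in sync.
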(event EventBeginPlay
  (bind _player_ref (Variables|Default|GetPlayer%20ref))
  (bind _grenadelauncher (Variables|/Game/Blueprints/FirstPersonBP/Blueprints/FirstPersonCharacter.FirstPersonCharacter_C|GetGrenadeLauncher _player_ref))
  (|CallParentFunction)
  (Variables|Default|SetAmmoCurrent (.ammocurrent _grenadelauncher))
  (Variables|Default|SetAmmoMax (.ammomax _grenadelauncher))
  (Variables|Default|SetClipSize (.clipsize _grenadelauncher)))

(event Collision|EventActorBeginOverlap
  (params (OtherActor :type Actor%20Object%20Reference))
  (|CallParentFunction OtherActor) ; This node is disabled and will not be called.\nDrag off pins to build functionality.
)

(event EventTick
  (params (DeltaSeconds :type Float%20%28single-precision%29))
  (|CallParentFunction DeltaSeconds) ; This node is disabled and will not be called.\nDrag off pins to build functionality.
)

(event EventStartShooting
  (|CallParentFunction)
  (CallFunction|FireBullet))

(event EventStopShooting
  (|CallParentFunction))

(fn ConstructionScript
  (|CallParentFunction))

(fn FireBullet
  (bind _player_ref (Variables|Default|GetPlayer%20ref))
  (|CallParentFunction)
  (bind _output_get (Variables|/Game/Blueprints/FirstPersonBP/Blueprints/FirstPersonCharacter.FirstPersonCharacter_C|SetGrenadeLauncher _player_ref (Utilities|Struct|MakeGunVariables "Gun_Glauncher_C" (Variables|Default|GetAmmoCurrent) (Variables|Default|GetAmmoMax) (Variables|Default|GetThumbnail) (Variables|Default|GetClipSize))))
  (Variables|/Game/Blueprints/FirstPersonBP/Blueprints/FirstPersonCharacter.FirstPersonCharacter_C|SetCurrentWeapon _player_ref _output_get))

(fn ReloadGun
  (bind _player_ref (Variables|Default|GetPlayer%20ref))
  (|CallParentFunction)
  (bind _output_get (Variables|/Game/Blueprints/FirstPersonBP/Blueprints/FirstPersonCharacter.FirstPersonCharacter_C|SetGrenadeLauncher _player_ref (Utilities|Struct|MakeGunVariables "Gun_Glauncher_C" (Variables|Default|GetAmmoCurrent) (Variables|Default|GetAmmoMax) (Variables|Default|GetThumbnail) (Variables|Default|GetClipSize))))
  (Variables|/Game/Blueprints/FirstPersonBP/Blueprints/FirstPersonCharacter.FirstPersonCharacter_C|SetCurrentWeapon _player_ref _output_get))