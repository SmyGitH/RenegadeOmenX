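; Base gun Blueprint, held as a child actor of FirstPersonCharacter, handling firing, ammo and reloading.
; FireBullet shoots from the camera as hitscan, single or randomized pellet spread, or launches an impulse-driven projectile, with montage, audio and muzzle flash.
; Tick stops shooting and auto-reloads on an empty magazine.
; Reload waits out the montage, then refills a clip at once or loops round by round for clipless guns.
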(event Custom|StartShooting
  (Variables|Default|SetisFiring true))

(event Custom|StopShooting
  (Variables|Default|SetisFiring false)
  (CallFunction|StopFiring))

(event Custom|Reload
  (if (not (Variables|Default|GetisFiring))
    (if (> (Variables|Default|GetAmmoMax) 0)
      (if (< (Variables|Default|GetAmmoCurrent) (Variables|Default|GetClipSize)) :!label _label
        (bind _delay (CallFunction|PerformReloadAnimation))
        (Utilities|FlowControl|Delay _delay)
        (CallFunction|ReloadGun)
        (Variables|Default|SetisReloading false)
        (if (not (Variables|Default|GethasClip))
          (if (<= (Variables|Default|GetAmmoCurrent) (Variables|Default|GetClipSize))
            (goto _label)))))))

(event EventBeginPlay
  (Audio|Components|Audio|Stop (Variables|Default|GetAudio))
  (bind _asfirst_person_character (Utilities|Casting|CastToFirstPersonCharacter (Game|GetPlayerCharacter 0)))
  (Variables|Default|SetPlayer%20ref _asfirst_person_character))

(event Collision|EventActorBeginOverlap
  (params (OtherActor :type Actor%20Object%20Reference)))

(event EventTick
  (params (DeltaSeconds :type Float%20%28single-precision%29))
  (if (<= (Variables|Default|GetAmmoCurrent) 0)
    (CallFunction|StopShooting)
    (if (not (<= (Variables|Default|GetAmmoMax) 0))
      (CallFunction|Reload))))

(fn ConstructionScript
  (Transformation|AttachComponentToComponent (Variables|Default|GetGunOffset) (Variables|Default|GetArms) "GunOffset" "SnapToTarget" "SnapToTarget" "SnapToTarget" true))

(fn FireBullet
  (if (Variables|Projectiles|GetisHitScan)
    (if (Variables|Default|GetisFireSpread)
      ;[1 1 1] Fires Pellet Spread
      (bind _asfirst_person_character (Utilities|Casting|CastToFirstPersonCharacter (Actor|GetParentActor)))
      (if (> (Variables|Default|GetAmmoCurrent) 0)
        (LocalVariables|SetGunDirection (Math|Vector|GetForwardVector (Transformation|GetWorldRotation (Variables|/Game/Blueprints/FirstPersonBP/Blueprints/FirstPersonCharacter.FirstPersonCharacter_C|GetFirstPersonCamera _asfirst_person_character))))
        (Utilities|FlowControl|Sequence
          (:then_0
            (for _index (range 0 5)
              (bind _outhit (Collision|LineTraceByChannel (Transformation|GetWorldLocation (Variables|/Game/Blueprints/FirstPersonBP/Blueprints/FirstPersonCharacter.FirstPersonCharacter_C|GetFirstPersonCamera _asfirst_person_character)) (Math|Vector|MakeVector (+ (.X (Math|Vector|BreakVector (+ (Transformation|GetWorldLocation (Variables|/Game/Blueprints/FirstPersonBP/Blueprints/FirstPersonCharacter.FirstPersonCharacter_C|GetFirstPersonCamera _asfirst_person_character)) (* (Math|Vector|GetForwardVector (Transformation|GetWorldRotation (Variables|/Game/Blueprints/FirstPersonBP/Blueprints/FirstPersonCharacter.FirstPersonCharacter_C|GetFirstPersonCamera _asfirst_person_character))) (Variables|Default|GetGunRange))))) (Math|Random|RandomFloatinRange -5e+01 5e+01)) (+ (.Y (Math|Vector|BreakVector (+ (Transformation|GetWorldLocation (Variables|/Game/Blueprints/FirstPersonBP/Blueprints/FirstPersonCharacter.FirstPersonCharacter_C|GetFirstPersonCamera _asfirst_person_character)) (* (Math|Vector|GetForwardVector (Transformation|GetWorldRotation (Variables|/Game/Blueprints/FirstPersonBP/Blueprints/FirstPersonCharacter.FirstPersonCharacter_C|GetFirstPersonCamera _asfirst_person_character))) (Variables|Default|GetGunRange))))) (Math|Random|RandomFloatinRange -5e+01 5e+01)) (+ (.Z (Math|Vector|BreakVector (+ (Transformation|GetWorldLocation (Variables|/Game/Blueprints/FirstPersonBP/Blueprints/FirstPersonCharacter.FirstPersonCharacter_C|GetFirstPersonCamera _asfirst_person_character)) (* (Math|Vector|GetForwardVector (Transformation|GetWorldRotation (Variables|/Game/Blueprints/FirstPersonBP/Blueprints/FirstPersonCharacter.FirstPersonCharacter_C|GetFirstPersonCamera _asfirst_person_character))) (Variables|Default|GetGunRange))))) (Math|Random|RandomFloatinRange -5e+01 5e+01))) "TraceTypeQuery1" false 0 "None"))
              (Class|AISenseDamage|ReportDamageEvent (.HitActor (Collision|BreakHitResult _outhit)) (Game|GetPlayerCharacter 0) 0.0 (.TraceStart (Collision|BreakHitResult _outhit)))
              (Game|Damage|ApplyDamage (.HitActor (Collision|BreakHitResult _outhit)) 1e+01 0 0)))
          (:then_1
            (Animation|Montage|MontagePlay (Components|SkeletalMesh|GetAnimInstance (Variables|Default|GetArms)) (Variables|Default|GetFireAnimation) (Variables|Default|GetFireRate) "MontageLength" 0.0 true)
            (Utilities|FlowControl|Sequence
              (:then_0
                (Audio|Components|Audio|Play (Variables|Default|GetAudio) 0.0)
                (Math|Integer|DecrementInt (Variables|Default|GetAmmoCurrent)))
              (:then_1
                (Rendering|SetVisibility (Variables|Default|GetMuzzleFlash) true false))))))
      (else
        ;[1 1 1] Fires Single Bullets
        (bind _asfirst_person_character_2 (Utilities|Casting|CastToFirstPersonCharacter (Actor|GetParentActor)))
        (if (> (Variables|Default|GetAmmoCurrent) 0)
          (LocalVariables|SetGunDirection (Math|Vector|GetForwardVector (Transformation|GetWorldRotation (Variables|/Game/Blueprints/FirstPersonBP/Blueprints/FirstPersonCharacter.FirstPersonCharacter_C|GetFirstPersonCamera _asfirst_person_character_2))))
          (bind _outhit_2 (Collision|LineTraceByChannel (Transformation|GetWorldLocation (Variables|/Game/Blueprints/FirstPersonBP/Blueprints/FirstPersonCharacter.FirstPersonCharacter_C|GetFirstPersonCamera _asfirst_person_character_2)) (+ (Transformation|GetWorldLocation (Variables|/Game/Blueprints/FirstPersonBP/Blueprints/FirstPersonCharacter.FirstPersonCharacter_C|GetFirstPersonCamera _asfirst_person_character_2)) (* (Math|Vector|GetForwardVector (Transformation|GetWorldRotation (Variables|/Game/Blueprints/FirstPersonBP/Blueprints/FirstPersonCharacter.FirstPersonCharacter_C|GetFirstPersonCamera _asfirst_person_character_2))) (Variables|Default|GetGunRange))) "TraceTypeQuery1" false 0 "None"))
          (Animation|Montage|MontagePlay (Components|SkeletalMesh|GetAnimInstance (Variables|Default|GetArms)) (Variables|Default|GetFireAnimation) 1.0 "MontageLength" 0.0 true :!label _label)
          (Utilities|FlowControl|Sequence
            (:then_0
              (Audio|Components|Audio|Play (Variables|Default|GetAudio) 0.0)
              (Math|Integer|DecrementInt (Variables|Default|GetAmmoCurrent)
                (:%20%20
                  (Class|AISenseDamage|ReportDamageEvent (.HitActor (Collision|BreakHitResult _outhit_2)) (Game|GetPlayerCharacter 0) 0.0 (.TraceStart (Collision|BreakHitResult _outhit_2)))
                  (Game|Damage|ApplyDamage (.HitActor (Collision|BreakHitResult _outhit_2)) 1e+01 0 0))))
            (:then_1
              (Rendering|SetVisibility (Variables|Default|GetMuzzleFlash) true false))))))
    (else
      ;[1 1 1] Fires Projectiles
      (bind _asfirst_person_character_3 (Utilities|Casting|CastToFirstPersonCharacter (Actor|GetParentActor)))
      (if (> (Variables|Default|GetAmmoCurrent) 0)
        (bind _returnvalue (Game|SpawnActorfromClass (Variables|Projectiles|GetProjectile) (Math|Transform|MakeTransform (+ (* (Math|Vector|GetForwardVector (Variables|/Game/Blueprints/FirstPersonBP/Blueprints/FirstPersonCharacter.FirstPersonCharacter_C|GetFirstPersonCamera _asfirst_person_character_3)) 1.5e+02) (Transformation|GetWorldLocation (Variables|/Game/Blueprints/FirstPersonBP/Blueprints/FirstPersonCharacter.FirstPersonCharacter_C|GetFirstPersonCamera _asfirst_person_character_3))) (Transformation|GetWorldRotation (Variables|/Game/Blueprints/FirstPersonBP/Blueprints/FirstPersonCharacter.FirstPersonCharacter_C|GetFirstPersonCamera _asfirst_person_character_3)) "0.200000,0.200000,0.200000") "AlwaysSpawn" 0 0))
        (Physics|AddImpulse (Variables|/Game/Blueprints/Guns/Grenade.Grenade_C|GetGrenade _returnvalue) (* (Math|Vector|GetForwardVector (Variables|/Game/Blueprints/FirstPersonBP/Blueprints/FirstPersonCharacter.FirstPersonCharacter_C|GetFirstPersonCamera _asfirst_person_character_3)) 3e+03) "None" true)
        (goto _label)))))

(fn ReloadGun
  (if (Variables|Default|GethasClip)
    (bind _output_get (LocalVariables|SetBulletDifference (- (Variables|Default|GetClipSize) (Variables|Default|GetAmmoCurrent))))
    (if (>= (Variables|Default|GetAmmoMax) _output_get)
      (Variables|Default|SetAmmoCurrent (Variables|Default|GetClipSize))
      (Variables|Default|SetAmmoMax (- (Variables|Default|GetAmmoMax) (LocalVariables|GetBulletDifference)))
      (else
        (Variables|Default|SetAmmoCurrent (+ (Variables|Default|GetAmmoCurrent) (Variables|Default|GetAmmoMax)))
        (Variables|Default|SetAmmoMax 0)))
    (else
      (Variables|Default|SetAmmoCurrent (+ (Variables|Default|GetAmmoCurrent) 1))
      (Variables|Default|SetAmmoMax (- (Variables|Default|GetAmmoMax) 1)))))

(fn StopFiring
  (Rendering|SetVisibility (Variables|Default|GetMuzzleFlash) false false)
  (Audio|Components|Audio|Stop (Variables|Default|GetAudio)))

(fn PerformReloadAnimation
  (if (Variables|Default|GethasClip)
    (if (not (Variables|Default|GetisReloading))
      (Variables|Default|SetisReloading true)
      (bind _returnvalue (Animation|Montage|MontagePlay (Components|SkeletalMesh|GetAnimInstance (Variables|Default|GetArms)) (Variables|Default|GetReloadAnimation) 1.0 "Duration" 0.0 true))
      (return _returnvalue))
    (elif (not (Variables|Default|GetisReloading))
      (Variables|Default|SetisReloading true)
      (bind _returnvalue_2 (Animation|Montage|MontagePlay (Components|SkeletalMesh|GetAnimInstance (Variables|Default|GetArms)) (Variables|Default|GetReloadAnimation) 2.0 "Duration" 0.0 true))
      (return _returnvalue_2))))