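; FindPathPoint is a behavior tree task that finds the current patrol point for a Zombie_Jill AI.
; It reads the path index from the Blackboard, picks that entry in the pawn's PatrolPath points and converts it from the path actor's local space to world space.
; It writes the result to the path vector key and finishes successfully, but never calls FinishExecute if the cast fails or the path is invalid.
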(event EventReceiveExecuteAI
  (params (OwnerController :type AI%20Controller%20Object%20Reference) (ControlledPawn :type Pawn%20Object%20Reference))
  (bind _aszombie_jill (Utilities|Casting|CastToZombie_Jill ControlledPawn))
  (bind _patrolpath (Variables|/Game/Blueprints/Zombies/Zombie_Jill.Zombie_Jill_C|GetPatrolPath _aszombie_jill)
    (:then
      (AI|BehaviorTree|SetBlackboardValueasVector (Variables|Default|GetBB_PathVector) (Math|Transform|TransformLocation (Transformation|GetActorTransform _patrolpath) (Utilities|Array|Get(acopy) (Variables|/Game/Blueprints/Zombies/PatrolPath.PatrolPath_C|GetPathPoints _patrolpath) (Class|BTFunctionLibrary|GetBlackboardValueasInt (Variables|Default|GetBB_PathIndex)))))
      (AI|BehaviorTree|FinishExecute true))
    (:else)))