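; Hideout entrance actor that banks the player's carried items as progress on overlap.
; When a FirstPersonCharacter enters, it loops over the inventory, adding item quantities to the character's Progress for slots passing an item class check.
; The inventory is cleared inside that loop, on each passing slot, rather than after it finishes.
; A sequence then saves player data through the game instance.
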(event Collision|EventActorBeginOverlap
  (params (OtherActor :type Actor%20Object%20Reference))
  (bind _asfirst_person_character (Utilities|Casting|CastToFirstPersonCharacter OtherActor))
  (Utilities|FlowControl|Sequence
    (:then_0
      (for _array_element (Variables|/Game/Blueprints/Inventory/InventoryComponent.InventoryComponent_C|GetInventory (Variables|/Game/Blueprints/FirstPersonBP/Blueprints/FirstPersonCharacter.FirstPersonCharacter_C|GetInventoryComponent _asfirst_person_character))
        (if (!= (.class (.itemstructure _array_element)) 0)
          (Variables|/Game/Blueprints/FirstPersonBP/Blueprints/FirstPersonCharacter.FirstPersonCharacter_C|SetProgress _asfirst_person_character (+ (.quantity _array_element) (Variables|/Game/Blueprints/FirstPersonBP/Blueprints/FirstPersonCharacter.FirstPersonCharacter_C|GetProgress _asfirst_person_character)))
          (Utilities|Array|Clear (Variables|/Game/Blueprints/Inventory/InventoryComponent.InventoryComponent_C|GetInventory (Variables|/Game/Blueprints/FirstPersonBP/Blueprints/FirstPersonCharacter.FirstPersonCharacter_C|GetInventoryComponent _asfirst_person_character))))))
    (:then_1
      (Default|SavePlayerData (Variables|/Game/Blueprints/FirstPersonBP/Blueprints/FirstPersonCharacter.FirstPersonCharacter_C|GetGameInstance _asfirst_person_character)))))

(fn ConstructionScript)