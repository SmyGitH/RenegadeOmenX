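; Hideout is a safehouse with entrance and exit overlap zones that show an interact prompt and let the player teleport between them.
; Interacting at the entrance converts supply items into Progress, saves player data, moves the player to the exit and destroys all zombies.
; Reaching 100 Progress then opens the win screen.
; Interacting at the exit returns the player to the entrance and activates the game mode's spawner.
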(event OnComponentBeginOverlap(Entrance)
  (params (OverlappedComponent :type Primitive%20Component%20Object%20Reference) (OtherActor :type Actor%20Object%20Reference) (OtherComp :type Primitive%20Component%20Object%20Reference) (OtherBodyIndex :type Integer) (bFromSweep :type Boolean) (SweepResult :type Hit%20Result%20Structure%20%28by%20ref%29))
  ;[1 1 1] Door interaction
  (Utilities|Casting|CastToRenegadeController OtherActor)
  (Variables|Default|SetatEntrance true)
  (bind _returnvalue (UserInterface|CreateWidget "/Game/Blueprints/FirstPersonBP/Blueprints/HUD/InteractUI.InteractUI_C"))
  (UserInterface|Viewport|AddtoViewport _returnvalue 0))

(event OnComponentBeginOverlap(Exit)
  (params (OverlappedComponent :type Primitive%20Component%20Object%20Reference) (OtherActor :type Actor%20Object%20Reference) (OtherComp :type Primitive%20Component%20Object%20Reference) (OtherBodyIndex :type Integer) (bFromSweep :type Boolean) (SweepResult :type Hit%20Result%20Structure%20%28by%20ref%29))
  ;[1 1 1] Door interaction
  (Utilities|Casting|CastToFirstPersonCharacter OtherActor)
  (Variables|Default|SetatExit true)
  (bind _returnvalue (UserInterface|CreateWidget "/Game/Blueprints/FirstPersonBP/Blueprints/HUD/InteractUI.InteractUI_C"))
  (UserInterface|Viewport|AddtoViewport _returnvalue 0))

(event OnComponentEndOverlap(Entrance)
  (params (OverlappedComponent :type Primitive%20Component%20Object%20Reference) (OtherActor :type Actor%20Object%20Reference) (OtherComp :type Primitive%20Component%20Object%20Reference) (OtherBodyIndex :type Integer))
  ;[1 1 1] Door interaction
  (Utilities|Casting|CastToFirstPersonCharacter OtherActor)
  (Variables|Default|SetatEntrance false)
  (Widget|RemovefromParent (stale OnComponentBeginOverlap(Entrance) _returnvalue)))

(event OnComponentEndOverlap(Exit)
  (params (OverlappedComponent :type Primitive%20Component%20Object%20Reference) (OtherActor :type Actor%20Object%20Reference) (OtherComp :type Primitive%20Component%20Object%20Reference) (OtherBodyIndex :type Integer))
  ;[1 1 1] Door interaction
  (Utilities|Casting|CastToFirstPersonCharacter OtherActor)
  (Variables|Default|SetatExit false)
  (Widget|RemovefromParent (stale OnComponentBeginOverlap(Exit) _returnvalue)))

(event EventInteract
  (params (Interaction :type Actor%20Object%20Reference))
  (bind _asfirst_person_character (Utilities|Casting|CastToFirstPersonCharacter Interaction))
  (if (Variables|Default|GetatEntrance)
    (Utilities|FlowControl|Sequence
      (:then_0
        (bind (_arrayindex _arrayelement) (Utilities|Array|ReverseforEachLoop (Variables|/Game/Blueprints/Inventory/InventoryComponent.InventoryComponent_C|GetInventory (Variables|/Game/Blueprints/FirstPersonBP/Blueprints/FirstPersonCharacter.FirstPersonCharacter_C|GetInventoryComponent _asfirst_person_character)))
          (:LoopBody
            (if (.issupply (.itemstructure _arrayelement))
              (Variables|/Game/Blueprints/FirstPersonBP/Blueprints/FirstPersonCharacter.FirstPersonCharacter_C|SetProgress _asfirst_person_character (+ (.quantity _arrayelement) (Variables|/Game/Blueprints/FirstPersonBP/Blueprints/FirstPersonCharacter.FirstPersonCharacter_C|GetProgress _asfirst_person_character)))
              (Utilities|Array|RemoveIndex (Variables|/Game/Blueprints/Inventory/InventoryComponent.InventoryComponent_C|GetInventory (Variables|/Game/Blueprints/FirstPersonBP/Blueprints/FirstPersonCharacter.FirstPersonCharacter_C|GetInventoryComponent _asfirst_person_character)) _arrayindex)))))
      (:then_1
        (Default|SavePlayerData (Variables|/Game/Blueprints/FirstPersonBP/Blueprints/FirstPersonCharacter.FirstPersonCharacter_C|GetGameInstance _asfirst_person_character)))
      (:then_2
        (Transformation|SetActorLocation _asfirst_person_character (Transformation|GetWorldLocation (Variables|Default|GetExit)) false false)
        (CallFunction|KillZombies))
      (:then_3
        (if (>= (Variables|/Game/Blueprints/FirstPersonBP/Blueprints/FirstPersonCharacter.FirstPersonCharacter_C|GetProgress _asfirst_person_character) 100)
          (Game|OpenLevel(byName) "You_Won_Screen"))))
    (elif (Variables|Default|GetatExit)
      (Transformation|SetActorLocation _asfirst_person_character (Transformation|GetWorldLocation (Variables|Default|GetEntrance)) false false)
      (Default|ActivateSpawner (.AsBP%20Game%20Mode%20Base (Utilities|Casting|CastToBP_GameMode_Base (Game|GetGameMode)))))))

(event EventBeginPlay)

(fn ConstructionScript)

(fn KillZombies
  (bind _outactors (Actor|GetAllActorsOfClass "/Game/Blueprints/Zombies/Zombie.Zombie_C"))
  (for _array_element _outactors
    (Actor|DestroyActor _array_element)))