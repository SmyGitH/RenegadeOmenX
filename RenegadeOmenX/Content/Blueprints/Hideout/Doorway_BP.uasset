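; Doorway actor in the Hideout folder that acts as a level-transition portal and banks the player's carried items as progress.
; On any trigger overlap, it adds item quantity to the character's Progress, clearing the inventory inside the loop at the first valid item.
; It then saves player data, records its DoorID in the game instance's save data, and opens the level named by its Destination enum.
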(event OnComponentBeginOverlap(PortalTrigger)
  (params (OverlappedComponent :type Primitive%20Component%20Object%20Reference) (OtherActor :type Actor%20Object%20Reference) (OtherComp :type Primitive%20Component%20Object%20Reference) (OtherBodyIndex :type Integer) (bFromSweep :type Boolean) (SweepResult :type Hit%20Result%20Structure%20%28by%20ref%29))
  (Utilities|FlowControl|Sequence
    (:then_0
      (bind _asfirst_person_character (Utilities|Casting|CastToFirstPersonCharacter (Game|GetPlayerCharacter 0)))
      (for _array_element (Variables|/Game/Blueprints/Inventory/InventoryComponent.InventoryComponent_C|GetInventory (Variables|/Game/Blueprints/FirstPersonBP/Blueprints/FirstPersonCharacter.FirstPersonCharacter_C|GetInventoryComponent _asfirst_person_character))
        (if (!= (.class (.itemstructure _array_element)) 0)
          (Variables|/Game/Blueprints/FirstPersonBP/Blueprints/FirstPersonCharacter.FirstPersonCharacter_C|SetProgress _asfirst_person_character (+ (.quantity _array_element) (Variables|/Game/Blueprints/FirstPersonBP/Blueprints/FirstPersonCharacter.FirstPersonCharacter_C|GetProgress _asfirst_person_character)))
          (Utilities|Array|Clear (Variables|/Game/Blueprints/Inventory/InventoryComponent.InventoryComponent_C|GetInventory (Variables|/Game/Blueprints/FirstPersonBP/Blueprints/FirstPersonCharacter.FirstPersonCharacter_C|GetInventoryComponent _asfirst_person_character))))))
    (:then_1
      (Default|SavePlayerData (Variables|/Game/Blueprints/FirstPersonBP/Blueprints/FirstPersonCharacter.FirstPersonCharacter_C|GetGameInstance _asfirst_person_character)))
    (:then_2
      (bind _asmy_game_instance (Utilities|Casting|CastToMyGameInstance (Game|GetGameInstance)))
      (Variables|/Game/Blueprints/Save_Load/SaveGameObject.SaveGameObject_C|SetDoorID (Variables|/Game/Blueprints/Save_Load/MyGameInstance.MyGameInstance_C|GetSaveGameData _asmy_game_instance) (Variables|Default|GetDoorID))
      (Game|OpenLevel(byName) (Utilities|String|StringToName (Utilities|String|EnumtoString (Variables|Default|GetDestination)))))))

(event Collision|EventActorBeginOverlap
  (params (OtherActor :type Actor%20Object%20Reference)))

(fn ConstructionScript)