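; Base gun actor for the first-person character, handling firing, ammo and reloading.
; FireBullet branches into hitscan pellet spread, single camera trace or spawned projectile, playing montage, audio and muzzle flash; traces draw persistent debug lines.
; The projectile branch rejoins the single-shot damage code, reading a trace it never runs.
; ReloadGun refills clips or adds single rounds; Start/StopShooting set IsFiring, while Tick stops effects when empty.
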(event Custom|StartShooting
  (Variables|Default|SetisFiring true))

(event Custom|StopShooting
  (Variables|Default|SetisFiring false)
  (CallFunction|StopFiring))

(event EventBeginPlay
  (Audio|Components|Audio|Stop (Variables|Default|GetAudio)))

(event Collision|EventActorBeginOverlap
  (params (OtherActor :type Actor%20Object%20Reference)))

(event EventTick
  (params (DeltaSeconds :type Float%20%28single-precision%29))
  (if (<= (Variables|Default|GetAmmoCurrent) 0)
    (CallFunction|StopFiring)))

(fn ConstructionScript
  (Transformation|AttachComponentToComponent (Variables|Default|GetGunOffset) (Variables|Default|GetArms) "GunOffset" "SnapToTarget" "SnapToTarget" "SnapToTarget" true))

(fn FireBullet
  (if (Variables|Projectiles|GetisHitScan)
    (if (Variables|Default|GetisFireSpread)
      ;[1 1 1] Fires Pellet Spread
      (bind _asfirst_person_character (Utilities|Casting|CastToFirstPersonCharacter (Actor|GetParentActor)))
      (if (> (Variables|Default|GetAmmoCurrent) 0)
        (LocalVariables|SetGunDirection (Math|Vector|GetForwardVector (Transformation|GetWorldRotation (Variables|/Game/Blueprints/FirstPersonBP/Blueprints/FirstPersonCharacter.FirstPersonCharacter_C|GetFirstPersonCamera _asfirst_person_character))))
        (Utilities|FlowControl|Sequence
          (:then_0
            (for _index (range 0 5)
              (bind _outhit (Collision|LineTraceByChannel (Transformation|GetWorldLocation (Variables|/Game/Blueprints/FirstPersonBP/Blueprints/FirstPersonCharacter.FirstPersonCharacter_C|GetFirstPersonCamera _asfirst_person_character)) (Math|Vector|MakeVector (+ (.X (Math|Vector|BreakVector (+ (Transformation|GetWorldLocation (Variables|/Game/Blueprints/FirstPersonBP/Blueprints/FirstPersonCharacter.FirstPersonCharacter_C|GetFirstPersonCamera _asfirst_person_character)) (* (Math|Vector|GetForwardVector (Transformation|GetWorldRotation (Variables|/Game/Blueprints/FirstPersonBP/Blueprints/FirstPersonCharacter.FirstPersonCharacter_C|GetFirstPersonCamera _asfirst_person_character))) (Variables|Default|GetGunRange))))) (Math|Random|RandomFloatinRange -1e+02 1e+02)) (+ (.Y (Math|Vector|BreakVector (+ (Transformation|GetWorldLocation (Variables|/Game/Blueprints/FirstPersonBP/Blueprints/FirstPersonCharacter.FirstPersonCharacter_C|GetFirstPersonCamera _asfirst_person_character)) (* (Math|Vector|GetForwardVector (Transformation|GetWorldRotation (Variables|/Game/Blueprints/FirstPersonBP/Blueprints/FirstPersonCharacter.FirstPersonCharacter_C|GetFirstPersonCamera _asfirst_person_character))) (Variables|Default|GetGunRange))))) (Math|Random|RandomFloatinRange -1e+02 1e+02)) (+ (.Z (Math|Vector|BreakVector (+ (Transformation|GetWorldLocation (Variables|/Game/Blueprints/FirstPersonBP/Blueprints/FirstPersonCharacter.FirstPersonCharacter_C|GetFirstPersonCamera _asfirst_person_character)) (* (Math|Vector|GetForwardVector (Transformation|GetWorldRotation (Variables|/Game/Blueprints/FirstPersonBP/Blueprints/FirstPersonCharacter.FirstPersonCharacter_C|GetFirstPersonCamera _asfirst_person_character))) (Variables|Default|GetGunRange))))) (Math|Random|RandomFloatinRange -1e+02 1e+02))) "TraceTypeQuery1" false 0 "Persistent"))
              (Class|AISenseDamage|ReportDamageEvent (.HitActor (Collision|BreakHitResult _outhit)) (Game|GetPlayerCharacter 0) 0.0 (.TraceStart (Collision|BreakHitResult _outhit)))
              (Game|Damage|ApplyDamage (.HitActor (Collision|BreakHitResult _outhit)) 1e+01 0 0)))
          (:then_1
            (Animation|Montage|MontagePlay (Components|SkeletalMesh|GetAnimInstance (Variables|Default|GetArms)) (Variables|Default|GetFireAnimation) (Variables|Default|GetFireRate) "MontageLength" 0.0 true)
            (Utilities|FlowControl|Sequence
              (:then_0
                (Audio|Components|Audio|Play (Variables|Default|GetAudio) 0.0)
                (Math|Integer|DecrementInt (Variables|Default|GetAmmoCurrent)))
              (:then_1
                (Rendering|SetVisibility (Variables|Default|GetMuzzleFlash) true false))))))
      (else
        ;[1 1 1] Fires Single Bullets
        (bind _asfirst_person_character_2 (Utilities|Casting|CastToFirstPersonCharacter (Actor|GetParentActor)))
        (if (> (Variables|Default|GetAmmoCurrent) 0)
          (LocalVariables|SetGunDirection (Math|Vector|GetForwardVector (Transformation|GetWorldRotation (Variables|/Game/Blueprints/FirstPersonBP/Blueprints/FirstPersonCharacter.FirstPersonCharacter_C|GetFirstPersonCamera _asfirst_person_character_2))))
          (bind _outhit_2 (Collision|LineTraceByChannel (Transformation|GetWorldLocation (Variables|/Game/Blueprints/FirstPersonBP/Blueprints/FirstPersonCharacter.FirstPersonCharacter_C|GetFirstPersonCamera _asfirst_person_character_2)) (+ (Transformation|GetWorldLocation (Variables|/Game/Blueprints/FirstPersonBP/Blueprints/FirstPersonCharacter.FirstPersonCharacter_C|GetFirstPersonCamera _asfirst_person_character_2)) (* (Math|Vector|GetForwardVector (Transformation|GetWorldRotation (Variables|/Game/Blueprints/FirstPersonBP/Blueprints/FirstPersonCharacter.FirstPersonCharacter_C|GetFirstPersonCamera _asfirst_person_character_2))) (Variables|Default|GetGunRange))) "TraceTypeQuery1" false 0 "Persistent"))
          (Animation|Montage|MontagePlay (Components|SkeletalMesh|GetAnimInstance (Variables|Default|GetArms)) (Variables|Default|GetFireAnimation) 1.0 "MontageLength" 0.0 true :!label _label)
          (Utilities|FlowControl|Sequence
            (:then_0
              (Audio|Components|Audio|Play (Variables|Default|GetAudio) 0.0)
              (Math|Integer|DecrementInt (Variables|Default|GetAmmoCurrent)
                (:%20%20
                  (Class|AISenseDamage|ReportDamageEvent (.HitActor (Collision|BreakHitResult _outhit_2)) (Game|GetPlayerCharacter 0) 0.0 (.TraceStart (Collision|BreakHitResult _outhit_2)))
                  (Game|Damage|ApplyDamage (.HitActor (Collision|BreakHitResult _outhit_2)) 1e+01 0 0))))
            (:then_1
              (Rendering|SetVisibility (Variables|Default|GetMuzzleFlash) true false))))))
    (else
      ;[1 1 1] Fires Projectiles
      (bind _asfirst_person_character_3 (Utilities|Casting|CastToFirstPersonCharacter (Actor|GetParentActor)))
      (if (> (Variables|Default|GetAmmoCurrent) 0)
        (Game|SpawnActorfromClass (Variables|Projectiles|GetProjectile) (Math|Transform|MakeTransform (Transformation|GetWorldLocation (Variables|Default|GetGunOffset)) (Transformation|GetWorldRotation (Variables|/Game/Blueprints/FirstPersonBP/Blueprints/FirstPersonCharacter.FirstPersonCharacter_C|GetFirstPersonCamera _asfirst_person_character_3)) "1,1,1") "Undefined" 0 0)
        (goto _label)))))

(fn ReloadGun
  (if (Variables|Default|GethasClip)
    (bind _output_get (LocalVariables|SetBulletDifference (- (Variables|Default|GetClipSize) (Variables|Default|GetAmmoCurrent))))
    (if (>= (Variables|Default|GetAmmoMax) _output_get)
      (Variables|Default|SetAmmoCurrent (Variables|Default|GetClipSize))
      (Variables|Default|SetAmmoMax (- (Variables|Default|GetAmmoMax) (LocalVariables|GetBulletDifference)))
      (else
        (Variables|Default|SetAmmoCurrent (+ (Variables|Default|GetAmmoCurrent) (Variables|Default|GetAmmoMax)))
        (Variables|Default|SetAmmoMax 0)))
    (elif (< (Variables|Default|GetAmmoCurrent) (Variables|Default|GetClipSize))
      (if (not (<= (Variables|Default|GetAmmoMax) 0))
        (Variables|Default|SetAmmoCurrent (+ (Variables|Default|GetAmmoCurrent) 1))
        (Variables|Default|SetAmmoMax (- (Variables|Default|GetAmmoMax) 1))))))

(fn StopFiring
  (Rendering|SetVisibility (Variables|Default|GetMuzzleFlash) false false)
  (Audio|Components|Audio|Stop (Variables|Default|GetAudio)))