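; Grenade actor that explodes the moment its Grenade component hits something.
; The hit spawns an enlarged explosion emitter, fires the RadialForce impulse, applies radial damage and destroys the actor.
; The damage radius is taken from the RadialForce's ImpulseStrength rather than its radius.
; A DamageMultiply helper scales Damage by a character's distance over Range, but the explosion does not call it.
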(event OnComponentHit(Grenade)
  (params (HitComponent :type Primitive%20Component%20Object%20Reference) (OtherActor :type Actor%20Object%20Reference) (OtherComp :type Primitive%20Component%20Object%20Reference) (NormalImpulse :type Vector :default "0, 0, 0") (Hit :type Hit%20Result%20Structure%20%28by%20ref%29))
  (Effects|SpawnEmitteratLocation "/Game/Assets/MobileStarterContent/Particles/P_Explosion.P_Explosion" (Transformation|GetActorLocation) "0, 0, 0" "10.000000,10.000000,10.000000")
  (Class|RadialForceComponent|FireImpulse (Variables|Default|GetRadialForce))
  (Game|Damage|ApplyRadialDamage (Variables|Default|GetDamage) (Transformation|GetWorldLocation (Variables|Default|GetGrenade)) (Variables|/Script/Engine.RadialForceComponent|GetImpulseStrength (Variables|Default|GetRadialForce)) 0 0 0 0 false "ECC_Visibility")
  (Actor|DestroyActor))

(event OnComponentBeginOverlap(Grenade)
  (params (OverlappedComponent :type Primitive%20Component%20Object%20Reference) (OtherActor :type Actor%20Object%20Reference) (OtherComp :type Primitive%20Component%20Object%20Reference) (OtherBodyIndex :type Integer) (bFromSweep :type Boolean) (SweepResult :type Hit%20Result%20Structure%20%28by%20ref%29)))

(event EventBeginPlay)

(fn ConstructionScript)

(fn DamageMultiply
  (params (Character :type Character%20Object%20Reference))
  (return (* (Math|Float|MapRangeClamped (Transformation|GetDistanceTo Character 0) 0.0 (Variables|Default|GetRange) 1.0 0.0) (Variables|Default|GetDamage))))